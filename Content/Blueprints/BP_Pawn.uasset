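; BP_Pawn is a player-controlled flying pawn that constantly moves forward and fires rockets.
; Tick feeds forward movement input, while the Pitch and Roll axes apply frame-rate-scaled local rotations to steer.
; Fire spawns a BP_Rocket at the Arrow component's transform.
; Holding Boost multiplies the FloatingPawnMovement max speed and acceleration, then divides them back on release.
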(event `self.ReceiveTick`
  (params (DeltaSeconds :type "Float (single-precision)"))
  (`self.AddMovementInput` (`self.GetActorForwardVector`)))

(event `InputAction|Fire`
  (params (Key :type "Key Structure"))
  (:`Pressed`
    (`|SpawnActorFromClass` "/Game/Blueprints/BP_Rocket.BP_Rocket_C" (`SceneComponent.K2_GetComponentToWorld` (`self.Arrow`)) "Undefined" "MultiplyWithRoot" null null)))

(event `InputAxis|Pitch`
  (params (AxisValue :type "Float (single-precision)"))
  (`self.K2_AddActorLocalRotation` (`KismetMathLibrary.MakeRotator` 0.0 (* AxisValue (`GameplayStatics.GetWorldDeltaSeconds`) 60.0))))

(event `InputAxis|Roll`
  (params (AxisValue :type "Float (single-precision)"))
  (`self.K2_AddActorLocalRotation` (`KismetMathLibrary.MakeRotator` (* AxisValue (`GameplayStatics.GetWorldDeltaSeconds`) 60.0))))

(event `InputAction|Boost`
  (params (Key :type "Key Structure"))
  (bind _floatingpawnmovement (`self.FloatingPawnMovement`))
  (bind _floatingpawnmovement_2 (`self.FloatingPawnMovement`))
  (bind _floatingpawnmovement_3 (`self.FloatingPawnMovement`))
  (bind _floatingpawnmovement_4 (`self.FloatingPawnMovement`))
  (:`Pressed`
    ; Start Boost
    (set `FloatingPawnMovement.MaxSpeed` (* (`FloatingPawnMovement.MaxSpeed` _floatingpawnmovement_3) 3.0) _floatingpawnmovement_3)
    (set `FloatingPawnMovement.Acceleration` (* (`FloatingPawnMovement.Acceleration` _floatingpawnmovement_4) 3.0) _floatingpawnmovement_4))
  (:`Released`
    ; Finish Boost
    (set `FloatingPawnMovement.MaxSpeed` (/ (`FloatingPawnMovement.MaxSpeed` _floatingpawnmovement_2) 3.0) _floatingpawnmovement_2)
    (set `FloatingPawnMovement.Acceleration` (/ (`FloatingPawnMovement.Acceleration` _floatingpawnmovement) 3.0) _floatingpawnmovement)))

(fn `UserConstructionScript`)